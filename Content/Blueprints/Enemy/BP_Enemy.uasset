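; BP_Enemy is a pawn that chases the player, deals damage on reaching them and dies when its health runs out.
; On BeginPlay it increments the game mode's alive count and starts PlayerChase, an AIMoveTo that damages the player on success and re-calls itself after a short delay.
; On death it decrements that count, calls CheckEnemyLeft, adds score, calls GotScore and destroys itself.
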(event `self.ReceiveAnyDamage`
  (params (Damage :type "Float (single-precision)") (DamageType :type "DamageType Object Reference") (InstigatedBy :type "Controller Object Reference") (DamageCauser :type "Actor Object Reference"))
  ;[1 1 1] Subtracts from health when damaged
  (bind _output_get (set `self.EnemyHealth` (- (`self.EnemyHealth`) Damage)))
  ;[1 1 1] Checks if enemy health is below 0
  (if (<= _output_get 0.0)
    ;[1 1 1] If enemy has 0 health or less
    ;;[1 1 1] Subtracts from enemies alive if enemy is killed
    (bind _asbp_first_person_game_mode (cast `/Game/FirstPerson/Blueprints/BP_FirstPersonGameMode` (`GameplayStatics.GetGameMode`)))
    (`/Engine/EditorBlueprintResources/StandardMacros.DecrementFloat` (`/Game/FirstPerson/Blueprints/BP_FirstPersonGameMode.EnemyAlive` _asbp_first_person_game_mode)
      (:`  `
        ;;[1 1 1] Call on Check Enemy Left event from BP_FirstPersonGamerMode which checks how many enemies are alive and if new ones need to spawm
        (`/Game/FirstPerson/Blueprints/BP_FirstPersonGameMode.CheckEnemyLeft` _asbp_first_person_game_mode)
        ;;[1 1 1] Adds score
        (set `/Game/FirstPerson/Blueprints/BP_FirstPersonGameMode.Score` (+ (`/Game/FirstPerson/Blueprints/BP_FirstPersonGameMode.Score` _asbp_first_person_game_mode) 5.0) _asbp_first_person_game_mode)
        ;;[1 1 1] Calls on Got Score event from BP_FirstPersonGameMode and adds to timer based on score
        (`/Game/FirstPerson/Blueprints/BP_FirstPersonGameMode.GotScore` _asbp_first_person_game_mode)
        ;;[1 1 1] Kills Enemy
        (`self.K2_DestroyActor`)))))

(event `PlayerChase`
  (params (PlayerToChase :type "Pawn Object Reference"))
  ;[1 1 1] AI moves to player
  (`|AIMoveTo` self (0.0 0.0 0.0) PlayerToChase 0.0
    (:`OnSuccess`
      ;[1 1 1] When AI reaches player it does damage to player
      (`GameplayStatics.ApplyDamage` PlayerToChase 10.0)
      (`KismetSystemLibrary.Delay` 0.2)
      (`self.PlayerChase` PlayerToChase))))

(event `self.ReceiveBeginPlay`
  ;[1 1 1] Adds to enemies alive counter
  (bind _asbp_first_person_game_mode (cast `/Game/FirstPerson/Blueprints/BP_FirstPersonGameMode` (`GameplayStatics.GetGameMode`)))
  (`/Engine/EditorBlueprintResources/StandardMacros.IncrementFloat` (`/Game/FirstPerson/Blueprints/BP_FirstPersonGameMode.EnemyAlive` _asbp_first_person_game_mode)
    (:`  `
      ;[1 1 1] Calls on Player Chase event
      (bind _asbp_first_person_character (cast `/Game/Blueprints/Character/BP_FirstPersonCharacter` (`GameplayStatics.GetPlayerCharacter` 0)))
      (`self.PlayerChase` _asbp_first_person_character))))

(fn `UserConstructionScript`)
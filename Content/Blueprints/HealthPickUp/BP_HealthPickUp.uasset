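; Health pickup that adds a fixed amount of health to the first-person player on overlap, with no maximum check.
; A Destroyed flag blocks repeat pickups and hides the actor, which reappears after a five-second delay instead of being destroyed.
; Tick feeds a Delay that acts as a throttle, periodically spawning the orb particle effect at the sphere while the pickup is visible.
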(event `self.Sphere1.OnComponentBeginOverlap`
  (params (OverlappedComponent :type "PrimitiveComponent Object Reference") (OtherActor :type "Actor Object Reference") (OtherComp :type "PrimitiveComponent Object Reference") (OtherBodyIndex :type Integer) (bFromSweep :type Boolean) (SweepResult :type "HitResult Structure (by ref)"))
  ;[1 1 1] When pick up collides with player it adds health to player if not hidden
  (bind _asbp_first_person_character (cast `/Game/Blueprints/Character/BP_FirstPersonCharacter` OtherActor))
  (if (not (`self.Destroyed`))
    (set `/Game/Blueprints/Character/BP_FirstPersonCharacter.PlayerHealth` (+ (`/Game/Blueprints/Character/BP_FirstPersonCharacter.PlayerHealth` _asbp_first_person_character) 25.0) _asbp_first_person_character)
    ;[1 1 1] Hides the pick up
    (set `self.Destroyed` true)
    (`self.SetActorHiddenInGame` (`self.Destroyed`))
    ;[1 1 1] Waits 5 seconds
    (`KismetSystemLibrary.Delay` 5.0)
    ;[1 1 1] Shows actor again
    (set `self.Destroyed` false)
    (`self.SetActorHiddenInGame` (`self.Destroyed`))))

(event `self.ReceiveTick`
  (params (DeltaSeconds :type "Float (single-precision)"))
  ;[1 1 1] Plays particle effect when pick up isn't hidden
  (`KismetSystemLibrary.Delay` 1.2)
  (if (not (`self.Destroyed`))
    (`GameplayStatics.SpawnEmitterAtLocation` "/Game/Effects/InfinityBladeEffects/Effects/FX_Archive/P_HealthOrb_Pickup.P_HealthOrb_Pickup" (`SceneComponent.K2_GetComponentLocation` (`self.Sphere`)))))

(fn `UserConstructionScript`)